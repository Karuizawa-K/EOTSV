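; BP_Cable is a spline-driven actor that builds a cable mesh along an editable spline.
; Its construction script calls SplineBuild, which adds a spline mesh component per spline point, bending it to the next point using local locations and tangents.
; Mesh, forward axis, mobility and material come from variables, and all segments share one dynamic material instance.
; The event graph holds no active logic.
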(fn `SplineBuild`
  (bind _spline (`self.Spline`))
  (bind _returnvalue (`KismetMaterialLibrary.CreateDynamicMaterialInstance` (`self.SplineMeshMaterial`)))
  (for _index (range (+ (`SplineComponent.GetNumberOfSplinePoints` _spline) 1))
    (bind _returnvalue_2 (`AddComponent|NODE_AddSplineMeshComponent-0` :`RelativeTransform` (`self.SplineMeshTransform`)))
    (`SplineMeshComponent.SetForwardAxis` _returnvalue_2 (`self.SplineMeshForwardAxis`) true)
    (`StaticMeshComponent.SetStaticMesh` _returnvalue_2 (`self.SplineMesh`))
    (`SceneComponent.SetMobility` _returnvalue_2 (`self.SplineMeshMobility`))
    (`PrimitiveComponent.SetMaterial` _returnvalue_2 0 _returnvalue)
    (`SceneComponent.K2_AttachToComponent` _returnvalue_2 _spline "None" "KeepRelative" "KeepRelative" "KeepRelative" true)
    (bind _returnvalue_3 (+ _index 1))
    (`SplineMeshComponent.SetStartAndEnd` _returnvalue_2 (`SplineComponent.GetLocationAtSplinePoint` _spline _index "Local") (`SplineComponent.GetTangentAtSplinePoint` _spline _index "Local") (`SplineComponent.GetLocationAtSplinePoint` _spline _returnvalue_3 "Local") (`SplineComponent.GetTangentAtSplinePoint` _spline _returnvalue_3 "Local") true)))

(fn `UserConstructionScript`
  (`self.SplineBuild`))